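; Base gameplay ability for line-trace ranged weapons, handling held-trigger fire, damage and effects.
; Activation starts a shot with montage; the locally controlled side traces and sets a timer from the weapon's FireDelay property.
; Input release flags the ability to end when firing completes, otherwise it fires again.
; Trace target data drives authority-only damage effects, plus fire cues and batched impact and last-bullet-hit trail cues.
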(event Custom|FireCompelete
  ;[1 1 1] 关于开火动作的逻辑
  (if (Variables|Default|GetbEndAbilityWhenCompelete)
    (Ability|EndAbility)
    (else
      (Utilities|FlowControl|Sequence
        (:then_0
          (Pawn|IsLocallyControlled
            (:True
              (Class|EquipmentGameplayAbilityTraceRangedWeapon|StartLineTrace)
              (Utilities|Time|SetTimerbyEvent (EventDispatchers|CreateEvent :!event Custom|FireCompelete) (Class|EquipmentInstance|GetFloatProperty (Class|EquipmentGameplayAbility|GetEquipmentInstance) "(TagName=\"Equipment.Property.FireDelay\")")))))
        (:then_1
          (|PlayMontageandWaitProxy "None" (Variables|Default|GetFireAnimationMontage) (Variables|Default|GetFireAnimationPlayRate) "None" true 1.0 0.0))))))

(event Ability|EventActivateAbility
  ;[1 1 1] 关于开火动作的逻辑
  (Variables|Default|SetbEndAbilityWhenCompelete false)
  (Ability|Tasks|WaitInputRelease false
    (:then
      (Class|ExpandedGameplayAbility|LocallyExecuteGameplayCueonOwner "(TagName=\"GameplayCue.Equipment.RangedWeapon.StartFire\")")
      (Utilities|FlowControl|Sequence
        (:then_0
          (Pawn|IsLocallyControlled
            (:True
              (Class|EquipmentGameplayAbilityTraceRangedWeapon|StartLineTrace)
              (Utilities|Time|SetTimerbyEvent (EventDispatchers|CreateEvent :!event Custom|FireCompelete) (Class|EquipmentInstance|GetFloatProperty (Class|EquipmentGameplayAbility|GetEquipmentInstance) "(TagName=\"Equipment.Property.FireDelay\")")))))
        (:then_1
          (|PlayMontageandWaitProxy "None" (Variables|Default|GetFireAnimationMontage) (Variables|Default|GetFireAnimationPlayRate) "None" true 1.0 0.0))))
    (:OnRelease
      (Variables|Default|SetbEndAbilityWhenCompelete true))))

(event Ability|EventOnEndAbility
  (params (bWasCancelled :type Boolean))
  (Class|EquipmentGameplayAbility|LocallyExecuteGameplayCueonVisualActor "(TagName=\"GameplayCue.Equipment.RangedWeapon.StopFire\")"))

(event EventOnLineTraceTargetDataReady
  (params (Data :type Gameplay%20Ability%20Target%20Data%20Handle%20Structure%20%28by%20ref%29))
  ;[1 1 1] 伤害判定（仅服务器）和视觉效果（多播）逻辑
  (Utilities|FlowControl|Sequence
    (:then_0
      (Class|EquipmentGameplayAbility|ExecuteGameplayCueonVisualActor "(TagName=\"GameplayCue.Equipment.RangedWeapon.Fire\")"))
    (:then_1
      (for _index (range 0 (- (Ability|TargetData|GetDataCountfromTargetData Data) 1))
        (Utilities|FlowControl|Sequence
          (:then_0
            (Ability|HasAuthority
              (:True
                (GameplayEffects|ApplyGameplayEffectToTarget Data (Variables|Default|GetInstantDamageEffectClass) 1 1) ; 在服务器上添加伤害Effect  TODO:支持同时施加多个效果
              )))
          (:then_1
            (Class|ExpandedGameplayAbility|AddBatchGameplayCueParamHitResult "(TagName=\"GameplayCue.Equipment.RangedWeapon.Impact.Batch\")" (Ability|TargetData|GetHitResultfromTargetData Data _index)))
          (:then_2
            (if (Class|EquipmentGameplayAbilityRangedWeapon|IsLastBulletHitResult Data _index)
              (Class|ExpandedGameplayAbility|AddBatchGameplayCueParamHitResult "(TagName=\"GameplayCue.Equipment.RangedWeapon.Trail.Batch\")" (Ability|TargetData|GetHitResultfromTargetData Data _index)))))))
    (:then_2
      (Class|EquipmentGameplayAbility|ExecuteGameplayCueonVisualActor "(TagName=\"GameplayCue.Equipment.RangedWeapon.Impact.Batch\")")
      (Class|EquipmentGameplayAbility|ExecuteGameplayCueonVisualActor "(TagName=\"GameplayCue.Equipment.RangedWeapon.Trail.Batch\")"))))